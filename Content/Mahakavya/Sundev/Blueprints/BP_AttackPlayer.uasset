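; Player character Blueprint for testing warrior attacks, with keyed light, normal, heavy, ability and three-step combo montages.
; Each attack locks input until completion, sets AttackNum and teleports BP_DamageWarrior to a world-X offset from the player.
; Mesh overlap with that warrior plays the damage montage matching AttackNum, gated by OnHit.
; It also has click-to-move outside battle and a Shift launch dash; PlayAnimationMontage is an empty stub.
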(event OnComponentBeginOverlap(Mesh)
  (params (OverlappedComponent :type Primitive%20Component%20Object%20Reference) (OtherActor :type Actor%20Object%20Reference) (OtherComp :type Primitive%20Component%20Object%20Reference) (OtherBodyIndex :type Integer) (bFromSweep :type Boolean) (SweepResult :type Hit%20Result%20Structure%20%28by%20ref%29))
  ;[1 1 1 1 25] EnemyDamage
  (if (Variables|Default|GetOn%20Hit)
    (bind _asbp_damage_warrior (Utilities|Casting|CastToBP_DamageWarrior OtherActor))
    (Variables|Default|SetOn%20Hit false)
    (switch int (Variables|Default|GetAttackNum)
      (:0
        (Animation|Montage|PlayMontage (Variables|/Script/Engine.Character|GetMesh _asbp_damage_warrior) "/Game/Mahakavya/Sundev/Animations/1st_Turn/1stTurnMontage/Turn1LDamage.Turn1LDamage"
          (:OnCompleted
            _)))
      (:1
        (Animation|Montage|PlayMontage (Variables|/Script/Engine.Character|GetMesh _asbp_damage_warrior) "/Game/Mahakavya/Sundev/Animations/1st_Turn/1stTurnMontage/Turn1NDamage.Turn1NDamage"
          (:OnCompleted
            _)))
      (:2
        (Animation|Montage|PlayMontage (Variables|/Script/Engine.Character|GetMesh _asbp_damage_warrior) "/Game/Mahakavya/Sundev/Animations/Hit/HitMontage/Warrior_Knockdown_Montage.Warrior_Knockdown_Montage"
          (:OnCompleted
            _)))
      (:3
        (Animation|Montage|PlayMontage (Variables|/Script/Engine.Character|GetMesh _asbp_damage_warrior) "/Game/Mahakavya/Sundev/Animations/3rd_Turn/3rdTurnMontage/Turn3DAbility.Turn3DAbility"
          (:OnCompleted
            _)))
      (:4
        (Animation|Montage|PlayMontage (Variables|/Script/Engine.Character|GetMesh _asbp_damage_warrior) "/Game/Mahakavya/Sundev/Animations/1st_Turn/1stTurnMontage/Heavy2Damage_Montage.Heavy2Damage_Montage"
          (:OnCompleted
            _)))
      (:5
        (Animation|Montage|PlayMontage (Variables|/Script/Engine.Character|GetMesh _asbp_damage_warrior) "/Game/Mahakavya/Sundev/Animations/2nd_Turn/2ndTurnMontage/Warrior_Damage_High_R_Montage.Warrior_Damage_High_R_Montage"
          (:OnCompleted
            _)))
      (:6
        (Animation|Montage|PlayMontage (Variables|/Script/Engine.Character|GetMesh _asbp_damage_warrior) "/Game/Mahakavya/Sundev/Animations/2nd_Turn/2ndTurnMontage/Warrior_Damage_High_L_Montage.Warrior_Damage_High_L_Montage"
          (:OnCompleted
            _)))
      (:7
        (Animation|Montage|PlayMontage (Variables|/Script/Engine.Character|GetMesh _asbp_damage_warrior) "/Game/Mahakavya/Sundev/Animations/2nd_Turn/2ndTurnMontage/Warrior_Damage_High_B_Montage.Warrior_Damage_High_B_Montage"
          (:OnCompleted
            _))))
    (Variables|Default|SetOn%20Hit true)))

(event Custom|Play%20Animation%20Montage
  ;[1 1 1] When the ui is ready
)

(event EventBeginPlay
  ;[1 1 1] Testing
  (Variables|/Script/Engine.PlayerController|SetbShowMouseCursor (Game|GetPlayerController 0) true)
  (bind _asgi_my_game_instance (Utilities|Casting|CastToGI_MyGameInstance (Game|GetGameInstance)))
  (Variables|GameData|SetGame%20Data _asgi_my_game_instance))

(event Input|MouseEvents|LeftMouseButton
  (params (Key :type Key%20Structure :default "None"))
  (bind _returnvalue (Game|GetPlayerController 0))
  (bind (_worldlocation _worlddirection) (Game|Player|ConvertMouseLocationToWorldSpace _returnvalue))
  ;[1 1 1] Testing
  (:Pressed
    (if (not (Variables|/Game/Mahakavya/RIP/Blueprints/GI_MyGameInstance.GI_MyGameInstance_C|GetIs%20In%20Battle (Variables|GameData|GetGame%20Data)))
      (bind (_outhit _returnvalue_2) (Collision|LineTraceByChannel _worldlocation (+ _worldlocation (* _worlddirection 1e+05)) "TraceTypeQuery1" false 0 "ForDuration"))
      (if _returnvalue_2
        (AI|Navigation|SimpleMovetoLocation (Game|GetPlayerController 0) (.Location (Collision|BreakHitResult _outhit)))))))

(event Input|KeyboardEvents|LeftAlt
  (params (Key :type Key%20Structure :default "None"))
  (bind _mesh (Variables|Character|GetMesh))
  ;[1 1 1] Attack
  (:Pressed
    (if (Variables|Default|GetAttackState)
      (Variables|Default|SetAttackState false)
      (switch int (Variables|Default|GetComboNum)
        (:0
          (Animation|Montage|PlayMontage _mesh "/Game/Mahakavya/Sundev/Animations/2nd_Turn/2ndTurnMontage/Warrior_Combo_3_1_Montage.Warrior_Combo_3_1_Montage"
            (:then
              (Variables|Default|SetAttackNum 5)
              (bind _returnvalue (Actor|GetActorOfClass "/Game/Mahakavya/Sundev/Blueprints/BP_DamageWarrior.BP_DamageWarrior_C" :!label _label))
              (Transformation|SetActorLocation _returnvalue (+ (Class|CharacterMovementComponent|GetLastUpdateLocation (Variables|Character|GetCharacterMovement)) "140.000000,0.000000,0.000000") false true))
            (:OnCompleted
              (Variables|Default|SetAttackState true))))
        (:1
          (Animation|Montage|PlayMontage _mesh "/Game/Mahakavya/Sundev/Animations/2nd_Turn/2ndTurnMontage/Warrior_Combo_3_2_Montage.Warrior_Combo_3_2_Montage"
            (:then
              (Variables|Default|SetAttackNum 6)
              (goto _label))
            (:OnCompleted
              (Variables|Default|SetAttackState true)
              (if (== (Variables|Default|GetComboNum) 2)
                (Variables|Default|SetComboNum 0)))))
        (:2
          (Animation|Montage|PlayMontage _mesh "/Game/Mahakavya/Sundev/Animations/2nd_Turn/2ndTurnMontage/Warrior_Combo_3_3_Montage.Warrior_Combo_3_3_Montage"
            (:then
              (Variables|Default|SetAttackNum 7)
              (goto _label))
            (:OnCompleted
              (Variables|Default|SetComboNum 0)
              (Variables|Default|SetAttackState true)))))
      (elif (Variables|Default|GetComboState)
        (if (== (Variables|Default|GetComboNum) 0)
          (Variables|Default|SetComboNum 1)
          (else
            (Variables|Default|SetComboNum 2)))))))

(event Input|KeyboardEvents|LeftShift
  (params (Key :type Key%20Structure :default "None"))
  ;[1 1 1] Testing
  (:Pressed
    (Character|LaunchCharacter (+ (* (Transformation|GetActorForwardVector) 2.5e+03) (* (Transformation|GetActorUpVector) 5e+01)) false false)))

(event Input|KeyboardEvents|1
  (params (Key :type Key%20Structure :default "None"))
  ;[1 1 1] Attack
  (:Pressed
    (if (Variables|Default|GetAttackState)
      (Variables|Default|SetAttackState false)
      (Animation|Montage|PlayMontage (Variables|Character|GetMesh) "/Game/Mahakavya/Sundev/Animations/1st_Turn/1stTurnMontage/Warrior_L_Attack_Montage.Warrior_L_Attack_Montage"
        (:then
          (Variables|Default|SetAttackNum 0)
          (bind _returnvalue (Actor|GetActorOfClass "/Game/Mahakavya/Sundev/Blueprints/BP_DamageWarrior.BP_DamageWarrior_C"))
          (Transformation|SetActorLocation _returnvalue (+ (Class|CharacterMovementComponent|GetLastUpdateLocation (Variables|Character|GetCharacterMovement)) "140.000000,0.000000,0.000000") false true))
        (:OnCompleted
          (Variables|Default|SetAttackState true))))))

(event Input|KeyboardEvents|3
  (params (Key :type Key%20Structure :default "None"))
  (bind _mesh (Variables|Character|GetMesh))
  (bind _charactermovement (Variables|Character|GetCharacterMovement))
  (bind _returnvalue (Class|CharacterMovementComponent|GetLastUpdateLocation _charactermovement))
  ;[1 1 1] Attack
  (:Pressed
    (if (Variables|Default|GetAttackState)
      (Variables|Default|SetAttackState false)
      (switch int 0
        (:Default
          (Animation|Montage|PlayMontage _mesh "/Game/Mahakavya/Sundev/Animations/1st_Turn/1stTurnMontage/Warrior_H_Attack_Montage.Warrior_H_Attack_Montage" :!label _label
            (:then
              (Variables|Default|SetAttackNum 2)
              (bind _returnvalue_2 (Actor|GetActorOfClass "/Game/Mahakavya/Sundev/Blueprints/BP_DamageWarrior.BP_DamageWarrior_C"))
              (Transformation|SetActorLocation _returnvalue_2 (+ _returnvalue "200.000000,0.000000,0.000000") false false))
            (:OnCompleted
              (Variables|Default|SetAttackState true))))
        (:0
          (goto _label))
        (:1
          (Animation|Montage|PlayMontage _mesh "/Game/Mahakavya/Sundev/Animations/3rd_Turn/3rdTurnMontage/Turn3HAttack.Turn3HAttack"
            (:then
              (Variables|Default|SetAttackNum 4)
              (bind _returnvalue_3 (Actor|GetActorOfClass "/Game/Mahakavya/Sundev/Blueprints/BP_DamageWarrior.BP_DamageWarrior_C"))
              (Transformation|SetActorLocation _returnvalue_3 (+ _returnvalue "140.000000,0.000000,0.000000") false true))
            (:OnCompleted
              (Variables|Default|SetAttackState true))))))))

(event Input|KeyboardEvents|2
  (params (Key :type Key%20Structure :default "None"))
  ;[1 1 1] Attack
  (:Pressed
    (if (Variables|Default|GetAttackState)
      (Variables|Default|SetAttackState false)
      (Animation|Montage|PlayMontage (Variables|Character|GetMesh) "/Game/Mahakavya/Sundev/Animations/1st_Turn/1stTurnMontage/Warrior_N_Attack_Montage.Warrior_N_Attack_Montage"
        (:then
          (Variables|Default|SetAttackNum 1)
          (bind _returnvalue (Actor|GetActorOfClass "/Game/Mahakavya/Sundev/Blueprints/BP_DamageWarrior.BP_DamageWarrior_C"))
          (Transformation|SetActorLocation _returnvalue (+ (Class|CharacterMovementComponent|GetLastUpdateLocation (Variables|Character|GetCharacterMovement)) "140.000000,0.000000,0.000000") false true))
        (:OnCompleted
          (Variables|Default|SetAttackState true))))))

(event Input|KeyboardEvents|LeftCtrl
  (params (Key :type Key%20Structure :default "None"))
  ;[1 1 1] Attack
  (:Pressed
    (if (Variables|Default|GetAttackState)
      (Variables|Default|SetAttackState false)
      (Animation|Montage|PlayMontage (Variables|Character|GetMesh) "/Game/Mahakavya/Sundev/Animations/3rd_Turn/3rdTurnMontage/Turn3Ability.Turn3Ability"
        (:then
          (Variables|Default|SetAttackNum 3)
          (bind _returnvalue (Actor|GetActorOfClass "/Game/Mahakavya/Sundev/Blueprints/BP_DamageWarrior.BP_DamageWarrior_C"))
          (Transformation|SetActorLocation _returnvalue (+ (Class|CharacterMovementComponent|GetLastUpdateLocation (Variables|Character|GetCharacterMovement)) "140.000000,0.000000,0.000000") false true))
        (:OnCompleted
          (Variables|Default|SetAttackState true))))))

(fn ConstructionScript)

(fn GetAnimationMontage
  (params (Montage%20Name :type E_Animations%20Enum :default "NewEnumerator0"))
  (for _array_element (Variables|Default|GetAnimation%20Montages)
    (if (Utilities|Enum|Equal(Enum) (Utilities|String|ToString(Object) _array_element) (Utilities|String|EnumtoString Montage%20Name))
      (return _array_element))))