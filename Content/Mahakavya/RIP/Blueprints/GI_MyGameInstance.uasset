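; Game instance that holds shared movement interpolation helpers and a per-turn action point counter.
; A stateful vector lerp advances alpha by delta time times a multiplier on each call, clamped to given bounds, with separate endpoint and reset setters.
; A 2D arrival check requires distance to exactly equal an offset.
; The action point setter stores the passed used amount minus the current value.
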(fn CustomLerpwithClamp
  (params (Clamp%20Minimum :type Float%20%28double-precision%29) (Clamp%20Maximum :type Float%20%28double-precision%29))
  (bind _output_get (Variables|LerpData|SetLerp%20Value (+ (Variables|LerpData|GetLerp%20Value) (* (Utilities|Time|GetWorldDeltaSeconds) (LocalVariables|GetLerp%20Multiplier)))))
  (return (Math|Vector|Lerp(Vector) (Variables|LerpData|GetLerp%20Start%20Value) (Variables|LerpData|GetLerp%20End%20Value) (Math|Float|Clamp(Float) _output_get Clamp%20Minimum Clamp%20Maximum))))

(fn SetLerpValue
  (params (Start%20Value :type Vector) (End%20Value :type Vector))
  (Variables|LerpData|SetLerp%20Start%20Value Start%20Value)
  (Variables|LerpData|SetLerp%20End%20Value End%20Value))

(fn ResetLerpValue
  (params (Default%20Lerp%20Value :type Float%20%28double-precision%29))
  (Variables|LerpData|SetLerp%20Value Default%20Lerp%20Value))

(fn ReachedDestinationV2D
  (params (Source :type Vector%202D%20Structure) (Target :type Vector%202D%20Structure) (Offset :type Float%20%28double-precision%29))
  (return (== (Math|Vector|Distance2D(Vector) Source Target) Offset)))

(fn RemainingActionPoints
  (return (Variables|GameData|GetAction%20Points%20Per%20Turn)))

(fn SetActionPoints
  (params (Action%20Point%20Used :type Integer))
  (Variables|GameData|SetAction%20Points%20Per%20Turn (- Action%20Point%20Used (Variables|GameData|GetAction%20Points%20Per%20Turn))))