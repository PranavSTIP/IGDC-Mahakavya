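; BP_TestPlayer is a test player character with click-to-move navigation and a forward dash.
; BeginPlay shows the mouse cursor and caches GI_MyGameInstance, whose IsInBattle flag blocks click movement during battle.
; A left click traces from the cursor on the Visibility channel, with debug drawing, and sends the character to the hit via SimpleMoveToLocation.
; Left Shift launches the character forward with slight lift, regardless of battle state.
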(event EventBeginPlay
  ;[1 1 1] Click to move
  (Variables|/Script/Engine.PlayerController|SetbShowMouseCursor (Game|GetPlayerController 0) true)
  (bind _asgi_my_game_instance (Utilities|Casting|CastToGI_MyGameInstance (Game|GetGameInstance)))
  (Variables|GameData|SetGame%20Data _asgi_my_game_instance))

(event Input|MouseEvents|LeftMouseButton
  (params (Key :type Key%20Structure :default "None"))
  ;[1 1 1] Click to move
  (:Pressed
    (if (not (Variables|/Game/Mahakavya/Blueprints/GI_MyGameInstance.GI_MyGameInstance_C|GetIs%20In%20Battle (Variables|GameData|GetGame%20Data)))
      (CallFunction|MovePlayer))))

(event Input|KeyboardEvents|LeftShift
  (params (Key :type Key%20Structure :default "None"))
  ;[1 1 1] Dash
  (:Pressed
    (Character|LaunchCharacter (+ (* (Transformation|GetActorForwardVector) 2.5e+03) (* (Transformation|GetActorUpVector) 5e+01)) false false)))

(fn ConstructionScript)

(fn MovePlayer
  (bind _returnvalue (Game|GetPlayerController 0))
  (bind (_worldlocation _worlddirection) (Game|Player|ConvertMouseLocationToWorldSpace _returnvalue))
  (bind (_outhit _returnvalue_2) (Collision|LineTraceByChannel _worldlocation (+ _worldlocation (* _worlddirection 1e+05)) "TraceTypeQuery1" false 0 "ForDuration"))
  (if _returnvalue_2
    (AI|Navigation|SimpleMovetoLocation (Game|GetPlayerController 0) (.Location (Collision|BreakHitResult _outhit)))))