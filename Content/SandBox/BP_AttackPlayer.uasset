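; Sandbox attack character that plays a warrior attack montage on the B key and a damage reaction on the warrior it touches.
; The key press also teleports a BP_DamageWarrior to a fixed world-X offset from this character's position.
; Mesh overlap with a BP_DamageWarrior plays that warrior's damage montage, with the ONHit flag blocking further hits until the montage completes.
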(event OnComponentBeginOverlap(Mesh)
  (params (OverlappedComponent :type Primitive%20Component%20Object%20Reference) (OtherActor :type Actor%20Object%20Reference) (OtherComp :type Primitive%20Component%20Object%20Reference) (OtherBodyIndex :type Integer) (bFromSweep :type Boolean) (SweepResult :type Hit%20Result%20Structure%20%28by%20ref%29))
  (Development|PrintString "Hello")
  (if (Variables|Default|GetONHit)
    (bind _asbp_damage_warrior (Utilities|Casting|CastToBP_DamageWarrior OtherActor))
    (Variables|Default|SetONHit false)
    (Animation|Montage|PlayMontage (Variables|/Script/Engine.Character|GetMesh _asbp_damage_warrior) "/Game/SandBox/DamageWarrior/Warrior_Damage_Anim_Montage.Warrior_Damage_Anim_Montage"
      (:OnCompleted
        (Variables|Default|SetONHit true)))))

(event EventBeginPlay)

(event Collision|EventActorBeginOverlap
  (params (OtherActor :type Actor%20Object%20Reference)))

(event EventTick
  (params (DeltaSeconds :type Float%20%28single-precision%29)))

(event Input|KeyboardEvents|B
  (params (Key :type Key%20Structure :default "None"))
  (:Pressed
    (Animation|Montage|PlayMontage (Variables|Character|GetMesh) "/Game/SandBox/AttackWarrior/warrior01__1__Anim_Montage.warrior01__1__Anim_Montage"
      (:then
        (bind _returnvalue (Actor|GetActorOfClass "/Game/SandBox/BP_DamageWarrior.BP_DamageWarrior_C"))
        (Transformation|SetActorLocation _returnvalue (+ (Class|CharacterMovementComponent|GetLastUpdateLocation (Variables|Character|GetCharacterMovement)) "150.000000,0.000000,0.000000") false false)))))

(fn ConstructionScript)